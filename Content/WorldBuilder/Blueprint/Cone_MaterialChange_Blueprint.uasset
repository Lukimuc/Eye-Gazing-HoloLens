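; Cone actor Blueprint in the WorldBuilder content with a point light whose color and brightness can be changed at runtime.
; The construction script sets the light to its starting intensity.
; One event applies a new color, and another maps a clamped alpha onto an intensity range that tops out at that starting value.
; Despite the MaterialChange name, the graphs contain no material logic.
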(event `/Game/WorldBuilder/Blueprint/Core/BPi_HoloLens.Update Light Color`
  (params (`New Color` :type "LinearColor Structure"))
  (`LightComponent.SetLightColor` (`self.PointLight`) `New Color` true))

(event `/Game/WorldBuilder/Blueprint/Core/BPi_HoloLens.Update Light Intensity`
  (params (Alpha :type "Float (double-precision)"))
  (`LightComponent.SetIntensity` (`self.PointLight`) (`KismetMathLibrary.MapRangeClamped` Alpha 0.0 1.0 0.0 (`self.StartingIntensity`))))

(fn `UserConstructionScript`
  (`LightComponent.SetIntensity` (`self.PointLight`) (`self.StartingIntensity`)))