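; AR player pawn for a hand- and voice-driven world builder, starting the AR session and UX Tools hand interactors one second after BeginPlay.
; Input actions toggle and drive BP_Toolbox, whose selection spawns from HeadTrackingHit, and also rotate a cube or enable puzzle-piece physics.
; Tracked geometry meshes are collected for an optional wireframe material.
; Tutorial head trace, eye gaze and hand-bone tracking remain but are disconnected from Tick.
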(event `ConfigureGestures`
  ;[0.1622 0.28 1] Basic Setup - That's what we need for the MetaHumans
  (`HeadMountedDisplayFunctionLibrary.ConfigureGestures` (make `XRGestureConfig` false true)))

(event `self.ReceiveBeginPlay`
  ;[0.1622 0.28 1] Basic Setup - That's what we need for the MetaHumans
  ;;[1 1 1] Event Triggers
  (`KismetSystemLibrary.K2_SetTimerDelegate` (delegate `WaitForTimer`) 1.0))

(event `WaitForTimer`
  ;[0.1622 0.28 1] Basic Setup - That's what we need for the MetaHumans
  ;;[1 1 1] Event Triggers
  (`self.PrepareForAR`))

(event `SpawnHandInteractions`
  (bind _returnvalue (`KismetMathLibrary.MakeTransform` (0.0 0.0 0.0)))
  ;[0.1622 0.28 1] Basic Setup - That's what we need for the MetaHumans
  ;;[1 1 1] Spawn a hand interaction for both hands
  (`|SpawnActorFromClass` "/Script/UXTools.UxtHandInteractionActor" _returnvalue "Undefined" "OverrideRootScale" self true "Left" null)
  (`|SpawnActorFromClass` "/Script/UXTools.UxtHandInteractionActor" _returnvalue "Undefined" "OverrideRootScale" self true "Right" null))

(event `PrepareForAR`
  ;[0.1622 0.28 1] Basic Setup - That's what we need for the MetaHumans
  ;;[1 1 1] Start AR Session & Set Location
  (`KismetSystemLibrary.PrintString` "Prepare For AR Called")
  (`ARBlueprintLibrary.StartARSession` "/Game/WorldBuilder/Assets/AR_SessionConfig_Custom.AR_SessionConfig_Custom")
  (`self.SpawnHandInteractions`)
  (`self.ConfigureGestures`))

(event `self.ReceiveEndPlay`
  (params (EndPlayReason :type "EEndPlayReason Enum" :default "Destroyed"))
  ;[0.1622 0.28 1] Basic Setup - That's what we need for the MetaHumans
  ;;[1 1 1] Start AR Session & Set Location
  (`ARBlueprintLibrary.StopARSession`))

(event `self.ReceiveTick`
  (params (DeltaSeconds :type "Float (single-precision)"))
  ;[1 0.5531 0.6915] Tutorial Logic - Not needed for MetaHumans
  ;;[1 1 1] Event Trigger
)

(event `HeadOrientationTracking`
  ;[1 0.5531 0.6915] Tutorial Logic - Not needed for MetaHumans
  ;;[1 1 1] HeadOrientation Tracking
  (bind _hmddata (`HeadMountedDisplayFunctionLibrary.GetHMDData` self))
  (if (break `XRHMDData` _hmddata)
    (bind _output_get (set `self.HMDData Position` (`.Position` (break `XRHMDData` _hmddata))))
    (bind _outhit (`KismetSystemLibrary.LineTraceSingle` :`Start` _output_get :`End` (+ _output_get (* (`KismetMathLibrary.GetForwardVector` (`KismetMathLibrary.Quat_Rotator` (`.Rotation` (break `XRHMDData` _hmddata)))) 500.0)) :`TraceChannel` "TraceTypeQuery1" :`DrawDebugType` "ForOneFrame" :`TraceColor` (struct :`G` 0.246696 :`B` 1.0 :`A` 1.0)))
    (set `self.HeadTrackingHit` _outhit)))

(event `EyeGazeTracking`
  (bind _hmddata_position (`self.HMDData Position`))
  ;[1 0.5531 0.6915] Tutorial Logic - Not needed for MetaHumans
  ;;[1 1 1] EyeTracking
  (if (`EyeTrackerFunctionLibrary.IsEyeTrackerConnected`)
    (bind (_outgazedata _returnvalue) (`EyeTrackerFunctionLibrary.GetGazeData`))
    (if _returnvalue
      (bind _outhit (`KismetSystemLibrary.LineTraceSingle` :`Start` _hmddata_position :`End` (+ _hmddata_position (* (`.GazeDirection` (break `EyeTrackerGazeData` _outgazedata)) 500.0)) :`TraceChannel` "TraceTypeQuery1" :`DrawDebugType` "ForOneFrame"))
      (bind (_bblockinghit _binitialoverlap _time _distance _location _impactpoint _normal _impactnormal _physmat _hitactor _hitcomponent) (`GameplayStatics.BreakHitResult` _outhit))
      (if _bblockinghit
        (bind _asbp_island_gaze (cast `/Game/WorldBuilder/Blueprint/BP_IslandGaze` _hitactor))
        (`/Game/WorldBuilder/Blueprint/BP_IslandGaze.ToggleGate` _asbp_island_gaze _hitcomponent)))))

(event `TrackHands`
  (bind _lefthand (`self.LeftHand`))
  ;[1 0.5531 0.6915] Tutorial Logic - Not needed for MetaHumans
  ;;[1 1 1] Hand Tracking
  (for _index (range 2)
    (bind _motioncontrollerdata (`HeadMountedDisplayFunctionLibrary.GetMotionControllerData` null (select `int` _index :`0` "Left" :`1` "Right" :!type "EControllerHand Enum")))
    (bind (_bvalid _devicename _applicationinstanceid _devicevisualtype _handindex _trackingstatus _gripposition _griprotation _aimposition _aimrotation _handkeypositions _handkeyrotations) (break `XRMotionControllerData` _motioncontrollerdata))
    (if (and _bvalid (`|EnumEquality` _devicevisualtype "Hand"))
      ;;[1 1 1] Retrieve the trackable points
      (bind _enumvalue (foreach `EHandKeypoint` false)
        (:`LoopBody`
          (bind _returnvalue (`self.RemoveSpaces` _enumvalue))
          (if (`SceneComponent.DoesSocketExist` (`self.RightHand`) _returnvalue)
            (switch `EControllerHand` _handindex
              (:`Left`
                (bind _returnvalue_2 (`HandKeypointConversion.Conv_HandKeypointToInt32` _enumvalue))
                (bind _returnvalue_3 (`KismetMathLibrary.MakeTransform` (`|GetArrayItem` _handkeypositions _returnvalue_2) (`KismetMathLibrary.Quat_Rotator` (`|GetArrayItem` _handkeyrotations _returnvalue_2))))
                (bind _adjustedtransform (`self.ConvertTransform` _returnvalue_3))
                (`PoseableMeshComponent.SetBoneTransformByName` _lefthand _returnvalue _adjustedtransform "ComponentSpace")
                (`SceneComponent.K2_SetWorldLocation` _lefthand (0.0 0.0 0.0) false false))
              (:`Right`
                (`PoseableMeshComponent.SetBoneTransformByName` (`self.RightHand`) _returnvalue _returnvalue_3 "WorldSpace")))))))))

(event `SpawnUI`
  ;[1 0.5531 0.6915] Tutorial Logic - Not needed for MetaHumans
  ;;[1 1 1] Handtracked UI
  (bind _returnvalue (`|SpawnActorFromClass` "/Game/WorldBuilder/Blueprint/UI/BP_ObjectSpawner.BP_ObjectSpawner_C" (`KismetMathLibrary.MakeTransform` (0.0 0.0 0.0)) "Undefined" "OverrideRootScale" self null))
  (add `/Game/WorldBuilder/Blueprint/UI/BP_ObjectSpawner.ObjectSpawnerActive` _returnvalue (delegate `UIHandsActive`)))

(event `UIHandsActive`
  (params (Active :type Boolean))
  ;[1 0.5531 0.6915] Tutorial Logic - Not needed for MetaHumans
  ;;[1 1 1] Handtracked UI
  (set `self.RenderHands` Active))

(event `InputAction|Rotate Cube`
  (params (Key :type "Key Structure"))
  (bind (_returnvalue_roll _returnvalue_pitch _returnvalue_yaw) (`KismetMathLibrary.BreakRotator` (`KismetMathLibrary.MakeRotator` 0.0 0.0 (+ (`self.Z_Rotation`) 20.0))))
  ;[1 0.5531 0.6915] Tutorial Logic - Not needed for MetaHumans
  ;;[1 1 1] Voice Input
  (:`Pressed`
    (`KismetSystemLibrary.PrintString` "Hello")
    (bind _returnvalue (`GameplayStatics.GetActorOfClass` "/Game/WorldBuilder/Blueprint/BP_RotateCube.BP_RotateCube_C"))
    (`SceneComponent.K2_SetRelativeRotation` (`Actor.RootComponent` _returnvalue) (`KismetMathLibrary.MakeRotator` 0.0 0.0 _returnvalue_yaw) false false)
    (set `self.Z_Rotation` _returnvalue_yaw)))

(event `InputAction|HL_WorldBuilder`
  (params (Key :type "Key Structure"))
  (bind _bp_toolbox (`self.BP_Toolbox`))
  ;[1 0.5531 0.6915] Tutorial Logic - Not needed for MetaHumans
  ;;[1 1 1] Voice Input
  (:`Pressed`
    (`/Engine/EditorBlueprintResources/StandardMacros.IsValid` _bp_toolbox
      (:`Is Valid`
        (`self.K2_DestroyActor` _bp_toolbox))
      (:`Is Not Valid`
        (bind _returnvalue (`|SpawnActorFromClass` "/Game/WorldBuilder/Blueprint/UI/BP_Toolbox.BP_Toolbox_C" (`KismetMathLibrary.MakeTransform` (0.0 0.0 0.0)) "Undefined" "OverrideRootScale" null null))
        (bind _output_get (set `self.BP_Toolbox` _returnvalue))
        (add `/Game/WorldBuilder/Blueprint/UI/BP_Toolbox.UserPressedSpawn` _output_get (delegate `UserPressendSpawn`))))))

(event `UserPressendSpawn`
  (params (ToSpawn :type "Actor Class Reference"))
  (bind (_headtrackinghit_bblockinghit _headtrackinghit_binitialoverlap _headtrackinghit_time _headtrackinghit_distance _headtrackinghit_location _headtrackinghit_impactpoint _headtrackinghit_normal _headtrackinghit_impactnormal _headtrackinghit_physmat _headtrackinghit_hitactor _headtrackinghit_hitcomponent _headtrackinghit_hitbonename _headtrackinghit_bonename _headtrackinghit_hititem _headtrackinghit_elementindex _headtrackinghit_faceindex _headtrackinghit_tracestart _headtrackinghit_traceend) (`GameplayStatics.BreakHitResult` (`self.HeadTrackingHit`)))
  ;[1 0.5531 0.6915] Tutorial Logic - Not needed for MetaHumans
  ;;[1 1 1] Voice Input
  (`|SpawnActorFromClass` ToSpawn (`KismetMathLibrary.MakeTransform` (+ _headtrackinghit_tracestart (* (`KismetMathLibrary.GetForwardVector` (`KismetMathLibrary.FindLookAtRotation` _headtrackinghit_tracestart _headtrackinghit_traceend)) 100.0))) "Undefined" "OverrideRootScale" null null)
  (`self.K2_DestroyActor` (`self.BP_Toolbox`)))

(event `InputAction|UI_Cube`
  (params (Key :type "Key Structure"))
  (bind _bp_toolbox (`self.BP_Toolbox`))
  ;[1 0.5531 0.6915] Tutorial Logic - Not needed for MetaHumans
  ;;[1 1 1] Voice Input
  ;;;[1 1 1] Voice mappings to interact with BP_Toolbox
  (:`Pressed`
    (`/Engine/EditorBlueprintResources/StandardMacros.IsValid` _bp_toolbox
      (:`Is Valid`
        (`/Game/WorldBuilder/Blueprint/UI/BP_Toolbox.Voice_SetSwitch` _bp_toolbox 0) ; 0 is a cube
      ))))

(event `InputAction|UI_Sphere`
  (params (Key :type "Key Structure"))
  (bind _bp_toolbox (`self.BP_Toolbox`))
  ;[1 0.5531 0.6915] Tutorial Logic - Not needed for MetaHumans
  ;;[1 1 1] Voice Input
  ;;;[1 1 1] Voice mappings to interact with BP_Toolbox
  (:`Pressed`
    (`/Engine/EditorBlueprintResources/StandardMacros.IsValid` _bp_toolbox
      (:`Is Valid`
        (`/Game/WorldBuilder/Blueprint/UI/BP_Toolbox.Voice_SetSwitch` _bp_toolbox 1) ; 1 is a sphere
      ))))

(event `InputAction|UI_Spawn`
  (params (Key :type "Key Structure"))
  (bind _bp_toolbox (`self.BP_Toolbox`))
  ;[1 0.5531 0.6915] Tutorial Logic - Not needed for MetaHumans
  ;;[1 1 1] Voice Input
  ;;;[1 1 1] Voice mappings to interact with BP_Toolbox
  (:`Pressed`
    (`/Engine/EditorBlueprintResources/StandardMacros.IsValid` _bp_toolbox
      (:`Is Valid`
        (`/Game/WorldBuilder/Blueprint/UI/BP_Toolbox.SpawnButtonPressed` _bp_toolbox null null)))))

(event `InputAction|Activate Physics`
  (params (Key :type "Key Structure"))
  ;[1 0.5531 0.6915] Tutorial Logic - Not needed for MetaHumans
  ;;[1 1 1] Voice Input
  (:`Pressed`
    (bind _returnvalue (`GameplayStatics.GetActorOfClass` "/Game/WorldBuilder/Blueprint/BP_PuzzlePiece.BP_PuzzlePiece_C"))
    (`PrimitiveComponent.SetSimulatePhysics` (`/Game/WorldBuilder/Blueprint/BP_PuzzlePiece.PuzzlePiece` _returnvalue) true)))

(event `self.ARTrackableNotify.OnUpdateTrackedGeometry`
  (params (TrackedGeometry :type "ARTrackedGeometry Object Reference"))
  (bind _returnvalue (`ARTrackedGeometry.GetUnderlyingMesh` TrackedGeometry))
  (bind (_returnvalue_additionalinfo _returnvalue_status) (break `ARSessionStatus` (`ARBlueprintLibrary.GetARSessionStatus`)))
  ;[1 0.5531 0.6915] Tutorial Logic - Not needed for MetaHumans
  ;;[1 1 1] Spatial Mapping
  (`/Engine/EditorBlueprintResources/StandardMacros.IsValid` _returnvalue
    (:`Is Valid`
      (if (`|EnumEquality` _returnvalue_status "Running")
        (bind _returnvalue_2 (`KismetArrayLibrary.Array_AddUnique` (`self.TrackedGeometry`) _returnvalue))
        (if (`self.SpacialMappingRenderMesh`)
          (`KismetSystemLibrary.PrintString` (`KismetStringLibrary.Conv_IntToString` _returnvalue_2))
          (`self.SpacialMappingSetVisibility` true))))))

(event `SpacialMappingSetVisibility`
  (params (Visible :type Boolean))
  (bind _trackedgeometry (`self.TrackedGeometry`))
  ;[1 0.5531 0.6915] Tutorial Logic - Not needed for MetaHumans
  ;;[1 1 1] Spatial Mapping
  (`KismetSystemLibrary.PrintString` "SpacialMappingSetVisibility called")
  (set `self.SpacialMappingRenderMesh` Visible)
  (for _array_element _trackedgeometry
    (`/Engine/EditorBlueprintResources/StandardMacros.IsValid` _array_element
      (:`Is Valid`
        (`PrimitiveComponent.SetMaterial` _array_element 0 (select `bool` (`self.SpacialMappingRenderMesh`) :`true` "/Game/WorldBuilder/Materials/Instance/M_EmissiveWire_Orange.M_EmissiveWire_Orange" :!type "MaterialInterface Object Reference")))
      (:`Is Not Valid`
        (`KismetArrayLibrary.Array_RemoveItem` _trackedgeometry _array_element)))))

(event `ToggleARSession`
  (params (Active :type Boolean))
  ;[1 0.5531 0.6915] Tutorial Logic - Not needed for MetaHumans
  ;;[1 1 1] Spatial Mapping
  (`KismetSystemLibrary.PrintString` "ToggleARSession called")
  (if Active
    (`ARBlueprintLibrary.StartARSession` "/Game/WorldBuilder/Assets/AR_SessionConfig_Custom.AR_SessionConfig_Custom")
    (`KismetSystemLibrary.PrintString` "AR Capture On" true true (struct :`G` 1.0 :`B` 0.083024 :`A` 1.0) 15.0)
    (else
      (`ARBlueprintLibrary.PauseARSession`)
      (`ARBlueprintLibrary.ToggleARCapture` false "SpatialMapping")
      (`KismetSystemLibrary.PrintString` "AR Capture Off" true true (struct :`R` 1.0 :`B` 0.261351 :`A` 1.0) 15.0))))

(event `self.ARTrackableNotify.OnAddTrackedGeometry`
  (params (TrackedGeometry :type "ARTrackedGeometry Object Reference"))
  ;[1 0.5531 0.6915] Tutorial Logic - Not needed for MetaHumans
  ;;[1 1 1] Spatial Mapping
)

(fn `ConvertTransform`
  (params (TrackedData :type "Transform Structure"))
  (returns (AdjustedTransform :type "Transform Structure"))
  (bind (_returnvalue_location _returnvalue_rotation _returnvalue_scale) (`KismetMathLibrary.BreakTransform` (`KismetMathLibrary.ComposeTransforms` TrackedData (`SceneComponent.K2_GetComponentToWorld` (`self.LeftHand`)))))
  (return (`KismetMathLibrary.MakeTransform` _returnvalue_location _returnvalue_rotation (* _returnvalue_scale (1.0 -1.0 1.0)))))

(fn `UserConstructionScript`)