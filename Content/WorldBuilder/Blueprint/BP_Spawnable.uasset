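; BP_Spawnable is a world-builder kit piece that shows a floor, ramp, wall or roof mesh chosen by ESpawnableType.
; SetAndPlaceMesh runs on construction and on CycleSpawnable, using component bounds to center the mesh horizontally with its top at the unshifted component location.
; CycleSpawnable only refreshes the mesh, ignoring its Up input.
; HasBeenSpawned adds a UXT Generic Manipulator component for interactive manipulation.
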(event `CycleSpawnable`
  (params (Up :type Boolean))
  (`self.Set and Place Mesh`))

(event `HasBeenSpawned`
  (`AddComponent|NODE_AddUxtGenericManipulatorComponent-0`))

(fn `Set and Place Mesh`
  (bind _staticmesh (`self.StaticMesh`))
  (bind _staticmesh_2 (`self.StaticMesh`))
  (bind (_origin _boxextent) (`KismetSystemLibrary.GetComponentBounds` _staticmesh_2))
  (`StaticMeshComponent.SetStaticMesh` _staticmesh (select `/Game/WorldBuilder/UI/Enums/ESpawnableType` (`self.ESpawnableType`) :`NewEnumerator0` "/Game/WorldBuilder/Assets/Architecture/Kit_Floor/Mesh/SM_Kit_Floor.SM_Kit_Floor" :`NewEnumerator1` "/Game/WorldBuilder/Assets/Architecture/Kit_Ramp/Mesh/SM_Kit_Ramp.SM_Kit_Ramp" :`NewEnumerator2` "/Game/WorldBuilder/Assets/Architecture/Kit_Wall/Mesh/SM_Kit_Wall_Straight.SM_Kit_Wall_Straight" :`NewEnumerator3` "/Game/WorldBuilder/Assets/Architecture/Kit_Roof/Mesh/SM_Kit_Roof_Corner_In.SM_Kit_Roof_Corner_In" :`NewEnumerator4` "/Game/WorldBuilder/Assets/Architecture/Kit_Roof/Mesh/SM_Kit_Roof_Corner_Out.SM_Kit_Roof_Corner_Out" :`NewEnumerator5` "/Game/WorldBuilder/Assets/Architecture/Kit_Roof/Mesh/SM_Kit_Roof_Straight.SM_Kit_Roof_Straight" :!type "StaticMesh Object Reference"))
  (`SceneComponent.K2_SetRelativeLocation` _staticmesh (0.0 0.0 0.0) false false)
  (`SceneComponent.K2_AddWorldOffset` _staticmesh_2 (- (- (`SceneComponent.K2_GetComponentLocation` _staticmesh_2) _origin) (`KismetMathLibrary.MakeVector` 0.0 0.0 (.z _boxextent))) false false))

(fn `UserConstructionScript`
  (`self.Set and Place Mesh`))